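; Pinball controller Blueprint that drives the left flippers in the level from player input.
; On BeginPlay it gathers every Flipper actor and sorts them into left and right arrays by FlipType.
; Pressing the LeftFlipper action prints a debug string and calls Flip on each left flipper, and releasing it calls Flop.
; The right flippers are collected, but no input here drives them.
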(event `self.ReceiveBeginPlay`
  (`self.DetectFlippers`))

(event `DetectFlippers`
  (bind _outactors (`GameplayStatics.GetAllActorsOfClass` "/Game/Padoru/Blueprints/Flipper.Flipper_C"))
  (for _array_element _outactors
    (switch `/Game/Padoru/Blueprints/FlipType` (`/Game/Padoru/Blueprints/Flipper.FlipType` _array_element)
      (:`NewEnumerator0`
        (`KismetArrayLibrary.Array_Add` (`self.RightFlippers`) _array_element))
      (:`NewEnumerator1`
        (`KismetArrayLibrary.Array_Add` (`self.LeftFlippers`) _array_element)))))

(event `InputAction|LeftFlipper`
  (params (Key :type "Key Structure"))
  (bind _leftflippers (`self.LeftFlippers`))
  (:`Pressed`
    (`KismetSystemLibrary.PrintString` "Hello")
    (for _array_element _leftflippers
      (`/Game/Padoru/Blueprints/Flipper.Flip` _array_element)))
  (:`Released`
    (for _array_element_2 _leftflippers
      (`/Game/Padoru/Blueprints/Flipper.Flop` _array_element_2))))

(fn `UserConstructionScript`)